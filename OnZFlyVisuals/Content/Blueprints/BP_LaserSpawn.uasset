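; BP_LaserSpawn spawns a BP_LaserModule at its own transform as a DMX-driven laser fixture.
; Each spawn disables mesh physics, passes on a DMX fixture patch and sets beam length.
; From BeginPlay, a self-calling delayed loop endlessly destroys and respawns the latest module.
; IA_SpawnLaser also triggers spawns; an event adds IMC_Rave, but the EnableInput call is unconnected.
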(event `Enable Input`
  (params (OldController :type "Controller Object Reference") (NewController :type "Controller Object Reference"))
  ; Input Mapping Context
  (bind _asplayer_controller (cast `PlayerController` NewController))
  (`EnhancedInputSubsystemInterface.AddMappingContext` (pcsubsystem `EnhancedInputLocalPlayerSubsystem` _asplayer_controller) "/Game/Blueprints/Rave_Inputs/Actions/IMC_Rave.IMC_Rave" 0 (struct)))

(event `self.ReceiveBeginPlay`
  (`|ExecutionSequence`
    (:`then_0`
      (`KismetSystemLibrary.Delay` 0.2)
      (`self.SpawnLaser`)
      (`self.LoopingSpawn`))))

(event `EnhancedInput|/Game/Blueprints/Rave_Inputs/Actions/IA_SpawnLaser`
  (params (ActionValue :type Boolean) (ElapsedSeconds :type "Float (double-precision)") (TriggeredSeconds :type "Float (double-precision)") (InputAction :type "InputAction Object Reference" :default "/Game/Blueprints/Rave_Inputs/Actions/IA_SpawnLaser.IA_SpawnLaser"))
  (:`Triggered`
    (`self.SpawnLaser` :!label _label))
  (:`Started`
    (goto _label)))

(event `SpawnLaser`
  (bind _returnvalue (`|SpawnActorFromClass` "/DMXFixtures/Laser/BP_LaserModule.BP_LaserModule_C" (`self.GetTransform`) "Undefined" "MultiplyWithRoot" null null))
  (`PrimitiveComponent.SetSimulatePhysics` (`/DMXFixtures/Laser/BP_LaserModule.SM_LaserModule` _returnvalue) false)
  (`|ExecutionSequence`
    (:`then_0`
      (`DMXComponent.SetFixturePatch` (`/DMXFixtures/Laser/BP_LaserModule.DMX` _returnvalue) (`|GetDMXFixturePatch` (struct :`DMXLibrary` "/Script/DMXRuntime.DMXLibrary'/Game/DMX_TD.DMX_TD'" :`bDisplayLibraryPicker` true :`EntityType` "/Script/CoreUObject.Class'/Script/DMXRuntime.DMXEntityFixturePatch'" :`EntityId` "EC1A02694D7F570C0D7AC69B2C2165D8")))
      (`KismetSystemLibrary.Delay` 0.2))
    (:`then_1`
      (set `/DMXFixtures/Laser/BP_LaserModule.BeamLength` 3000.0 _returnvalue))))

(event `LoopingSpawn`
  (`self.K2_DestroyActor` (stale `SpawnLaser` _returnvalue))
  (`KismetSystemLibrary.Delay` 0.2)
  (`self.SpawnLaser`)
  (`KismetSystemLibrary.Delay` 0.2)
  (`self.LoopingSpawn`))

(fn `UserConstructionScript`)